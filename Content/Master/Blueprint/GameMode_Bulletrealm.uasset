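; Game mode for Bulletrealm that spawns a character for each player at a saved PlayerStart, up to a player limit.
; SavePlayersStartPosition caches the transforms of all PlayerStart actors.
; CreateNewCharacter takes the next index from a player counter, printing a warning once the maximum is exceeded.
; SpawnCharacter then, on authority only, spawns the given class at that index's transform, possesses it and stores the index on the PlayerController_Generic.
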(fn ConstructionScript)

(fn SavePlayersStartPosition
  ;[1 1 1] Saving Player Start Positions
  (bind _outactors (Actor|GetAllActorsOfClass "/Script/Engine.PlayerStart"))
  (for _array_element _outactors
    (Utilities|Array|Add (Variables|Properties|GetARSaveStartPlayerPositions) (Transformation|GetActorTransform _array_element))))

(fn CreateNewPlayerIndex
  (if (<= (Variables|CurrentState|GetPlayerCountNum) (Variables|DefaultValue|GetPlayerMaxAllowed))
    (bind _output_get (Variables|CurrentState|SetPlayerCountNum (+ (Variables|CurrentState|GetPlayerCountNum) 1)))
    (return (<= (Variables|CurrentState|GetPlayerCountNum) (Variables|DefaultValue|GetPlayerMaxAllowed)) (- _output_get 1))))

(fn CreateNewCharacter
  (params (InputController :type Player%20Controller%20Object%20Reference) (CharacterClass :type Character%20Generic%20Class%20Reference))
  (bind (_creationallowed _playerindex) (CallFunction|CreateNewPlayerIndex))
  (if _creationallowed
    (bind _asplayer_controller_generic (Utilities|Casting|CastToPlayerController_Generic InputController))
    (bind _resultcharacter (CallFunction|SpawnCharacter CharacterClass _playerindex _asplayer_controller_generic))
    (return _resultcharacter)
    (else
      (Development|PrintString "Maximum player exceeds" true false "(R=0.510000,G=0.027644,B=0.088699,A=1.000000)" 1e+01))))

(fn SpawnCharacter
  (params (CharacterClass :type Character%20Generic%20Class%20Reference) (InputIndex :type Integer) (InputController :type Player%20Controller%20Object%20Reference))
  (Utilities|IsValid InputController
    (:Is%20Valid
      (Networking|SwitchHasAuthority
        (:Authority
          (bind _returnvalue (Game|SpawnActorfromClass CharacterClass (Utilities|Array|Get(acopy) (Variables|Properties|GetARSaveStartPlayerPositions) InputIndex) "Undefined" InputController 0))
          (Utilities|IsValid _returnvalue
            (:Is%20Valid
              (Pawn|Possess InputController _returnvalue)
              (bind _asplayer_controller_generic (Utilities|Casting|CastToPlayerController_Generic InputController))
              (Variables|/Game/Master/Blueprint/PlayerController_Generic.PlayerController_Generic_C|SetMyIndex _asplayer_controller_generic InputIndex)
              (return _returnvalue))))))))