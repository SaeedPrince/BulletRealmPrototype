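; Player controller, named for an entry stage, that sets up save data and toggles a network menu.
; On BeginPlay it loads the save game from its slot, or creates a new instance without writing it.
; The NetWorkMenu input flip-flops between MenuShow and MenuHide, which add or remove the widget and toggle the mouse cursor.
; MenuShow reuses the cached widget, creating one only when it is invalid or of another class.
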(event EventBeginPlay
  (bind _savefile (Variables|Game|GetSaveFile))
  ;[1 1 1] Assigning game objects at begin play
  (bind _returnvalue (SaveGame|DoesSaveGameExist _savefile))
  (if _returnvalue
    (bind _returnvalue_2 (SaveGame|LoadGamefromSlot _savefile))
    (Variables|Game|SetbpSaveGameInstance _returnvalue_2)
    (else
      (bind _returnvalue_3 (SaveGame|CreateSaveGameObject "/Game/Master/Blueprint/BP_SaveGame.BP_SaveGame_C"))
      (Variables|Game|SetbpSaveGameInstance _returnvalue_3))))

(event Input|ActionEvents|InputActionNetWorkMenu
  (params (Key :type Key%20Structure :default "AnyKey"))
  ;[1 1 1] Network Menu
  (:Pressed
    (Utilities|FlowControl|FlipFlop
      (:A
        (CallFunction|MenuShow "/Game/Master/Blueprint/MenuNetwork.MenuNetwork_C"))
      (:B
        (CallFunction|MenuHide)))))

(fn ConstructionScript)

(fn MenuShow
  (params (MenuClass :type User%20Widget%20Class%20Reference))
  (Utilities|IsValid (Variables|Game|GetScreenMenu)
    (:Is%20Valid
      (if (== (Utilities|GetClass (Variables|Game|GetScreenMenu)) MenuClass)
        _
        (else
          (bind _returnvalue (UserInterface|CreateWidget MenuClass self :!label _label))
          (bind _output_get (Variables|Game|SetScreenMenu _returnvalue)))))
    (:Is%20Not%20Valid
      (goto _label)))
  (UserInterface|Viewport|AddtoViewport _output_get 0)
  (Variables|/Script/Engine.PlayerController|SetbShowMouseCursor self true))

(fn MenuHide
  (Widget|RemovefromParent (Variables|Game|GetScreenMenu))
  (Variables|/Script/Engine.PlayerController|SetbShowMouseCursor self false))