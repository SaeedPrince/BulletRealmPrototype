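; Generic player controller Blueprint that requests character spawns and manages a single on-screen menu widget.
; On the server, it caches the ArenaSmall game mode at BeginPlay and has it create a Character_Generic on request, linking character and controller.
; MenuShow reuses or recreates the widget by class and adds it to the viewport.
; MenuHide removes it and hides the cursor, though the cursor-show step in MenuShow is disconnected.
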(event Custom|RequestSpawnCharacterOnServer
  ;[1 1 1] Request Character Spawn On Server
  (bind _asgame_mode_arena_small (Utilities|Casting|CastToGameMode_ArenaSmall (Game|GetGameMode)))
  (bind _resultcharacter (Default|CreateNewCharacter _asgame_mode_arena_small self "/Game/Master/Blueprint/Character_Generic.Character_Generic_C"))
  (Utilities|IsValid _resultcharacter
    (:Is%20Valid
      (bind _output_get (Variables|GameObject|SetCharacterBP _resultcharacter))
      (Variables|/Game/Master/Blueprint/Character_Generic.Character_Generic_C|SetPlController _output_get self))))

(event EventBeginPlay
  ;[1 1 1] Begin play
  (Networking|SwitchHasAuthority
    (:Authority
      (bind _asgame_mode_arena_small (Utilities|Casting|CastToGameMode_ArenaSmall (Game|GetGameMode)))
      (Variables|GameObject|SetTheGameMode _asgame_mode_arena_small))))

(fn ConstructionScript)

(fn MenuShow
  (params (MenuClass :type User%20Widget%20Class%20Reference))
  (Utilities|IsValid (Variables|Menu|GetScreenMenu)
    (:Is%20Valid
      (if (== (Utilities|GetClass (Variables|Menu|GetScreenMenu)) MenuClass)
        _
        (else
          (bind _returnvalue (UserInterface|CreateWidget MenuClass self :!label _label))
          (bind _output_get (Variables|Menu|SetScreenMenu _returnvalue)))))
    (:Is%20Not%20Valid
      (goto _label)))
  (UserInterface|Viewport|AddtoViewport _output_get 0))

(fn MenuHide
  (Widget|RemovefromParent (Variables|Menu|GetScreenMenu))
  (Variables|/Script/Engine.PlayerController|SetbShowMouseCursor self false))